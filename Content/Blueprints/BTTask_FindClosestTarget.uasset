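; Behavior tree task that finds the Building actor nearest to the AI's controlled pawn and stores its location as the target.
; On execute, it loops over every Building in the level, keeping the shortest distance and that actor's location.
; It writes the location to the TargetLocation blackboard key.
; Success depends on the validity of the last looped element, not on the stored nearest result.
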(event `self.ReceiveExecute`
  (params (OwnerActor :type "Actor Object Reference"))
  (bind _returnvalue (`AIBlueprintHelperLibrary.GetAIController` OwnerActor))
  (set `self.NearestDistance` 99999999.0)
  (bind _outactors (`GameplayStatics.GetAllActorsOfClass` "/Script/Jan24.Building"))
  (for _array_element _outactors
    (bind _returnvalue_2 (`Actor.GetDistanceTo` (`Controller.K2_GetPawn` _returnvalue) _array_element))
    (if (< _returnvalue_2 (`self.NearestDistance`))
      (set `self.NearestDistance` _returnvalue_2)
      (set `self.Nearest` (.location (`Actor.GetTransform` _array_element)))))
  (`BlackboardComponent.SetValueAsVector` (`AIBlueprintHelperLibrary.GetBlackboard` _returnvalue) (`KismetStringLibrary.Conv_StringToName` "TargetLocation") (`self.Nearest`))
  (`self.FinishExecute` (`KismetSystemLibrary.IsValid` _array_element)))