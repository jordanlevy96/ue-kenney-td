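; Player controller that sets up the in-game menu and drives building placement previews.
; On BeginPlay it adds the player input mapping context and creates the InGameMenu widget on the viewport.
; Each Tick, while a ghost building exists, it traces from the mouse cursor into the world and snaps the ghost to the hit point at ground height zero.
; The ghost then checks collisions, given valid and invalid ghost materials.
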(event `self.ReceiveBeginPlay`
  (`EnhancedInputSubsystemInterface.AddMappingContext` (subsystem `EnhancedInputLocalPlayerSubsystem`) "/Game/Inputs/PlayerInputContext.PlayerInputContext" 0 (struct))
  (bind _returnvalue (`|CreateWidget` "/Game/UI/InGameMenu.InGameMenu_C"))
  (`UserWidget.AddToViewport` _returnvalue 0))

(event `self.ReceiveTick`
  (params (DeltaSeconds :type "Float (single-precision)"))
  (bind (_locationx _locationy) (`self.GetMousePosition`))
  (bind _ghostbuilding (`self.GhostBuilding`))
  (bind (_worldposition _worlddirection) (`GameplayStatics.DeprojectScreenToWorld` self (`KismetMathLibrary.MakeVector2D` _locationx _locationy)))
  (if (`KismetSystemLibrary.IsValid` _ghostbuilding)
    (bind _outhit (`KismetSystemLibrary.LineTraceSingle` _worldposition (+ _worldposition (* _worlddirection 100000.0)) "TraceTypeQuery1"))
    (`self.K2_SetActorLocation` _ghostbuilding (`KismetMathLibrary.MakeVector` (.x (`.Location` (`GameplayStatics.BreakHitResult` _outhit))) (.y (`.Location` (`GameplayStatics.BreakHitResult` _outhit)))) false true)
    (`GhostBuilding.CheckForCollisions` _ghostbuilding "/Game/M_Ghost.M_Ghost" "/Game/M_GhostInvalid.M_GhostInvalid")))

(fn `UserConstructionScript`)